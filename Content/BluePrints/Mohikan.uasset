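; Mohikan is an enemy character that turns its capsule toward the player every tick and chases them.
; A Sphere overlap starts the AIMoveTo chase, and an Attack overlap pauses it until the player leaves.
; The attack state only runs a half-second delay, with no action after it.
; It binds to the player's HitEvent dispatcher to print "damage" and play a flinch animation.
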(event `self.ReceiveBeginPlay`
  (bind _asthird_person_character (cast `/Game/BluePrints/ThirdPersonCharacter` (`GameplayStatics.GetPlayerPawn` 0)))
  (add `/Game/BluePrints/ThirdPersonCharacter.HitEvent` _asthird_person_character (delegate `Damage_Event`)))

(event `Damage_Event`
  (`KismetSystemLibrary.PrintString` "damage")
  (`SkeletalMeshComponent.PlayAnimation` (`self.Mesh`) "/Game/Model/mohiAnim/mohi-_hirumi.mohi-_hirumi" false))

(event `self.ReceiveTick`
  (params (DeltaSeconds :type "Float (single-precision)"))
  (bind _returnvalue (`GameplayStatics.GetPlayerPawn` 0))
  (`|ExecutionSequence`
    (:`then_0`
      (`SceneComponent.K2_SetWorldRotation` (`self.CapsuleComponent`) (`KismetMathLibrary.MakeRotator` 0.0 0.0 (.yaw (`KismetMathLibrary.FindLookAtRotation` (`self.K2_GetActorLocation`) (`self.K2_GetActorLocation` _returnvalue)))) false false))
    (:`then_1`
      (if (`self.isDiscover`)
        (`|AIMoveTo` self (0.0 0.0 0.0) _returnvalue 125.0 true)))
    (:`then_2`
      (if (`self.isAttack`)
        (`KismetSystemLibrary.Delay` 0.5)))))

(event `self.Sphere.OnComponentBeginOverlap`
  (params (OtherActor :type "Actor Object Reference") (OtherComp :type "PrimitiveComponent Object Reference") (OtherBodyIndex :type Integer) (bFromSweep :type Boolean) (SweepResult :type "HitResult Structure (by ref)"))
  (if (== OtherActor (`GameplayStatics.GetPlayerPawn` 0))
    (set `self.isDiscover` true)))

(event `self.Attack.OnComponentBeginOverlap`
  (params (OtherActor :type "Actor Object Reference") (OtherComp :type "PrimitiveComponent Object Reference") (OtherBodyIndex :type Integer) (bFromSweep :type Boolean) (SweepResult :type "HitResult Structure (by ref)"))
  (if (== OtherActor (`GameplayStatics.GetPlayerPawn` 0))
    (set `self.isAttack` true)
    (set `self.isDiscover` false)))

(event `self.Attack.OnComponentEndOverlap`
  (params (OtherActor :type "Actor Object Reference") (OtherComp :type "PrimitiveComponent Object Reference") (OtherBodyIndex :type Integer))
  (if (== OtherActor (`GameplayStatics.GetPlayerPawn` 0))
    (set `self.isAttack` false)
    (set `self.isDiscover` true)))

(fn `UserConstructionScript`)