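; Lovers is an actor with a skeletal mesh that responds to hugs from the player's ThirdPersonCharacter.
; On BeginPlay it plays a wait animation and passes its hug-start and hug-end events to that character.
; These events switch between hug and finish animations and toggle a flag that makes Tick yaw the actor toward the player.
; Logic to step the mesh while the player is distant is left unconnected.
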(event `self.ReceiveBeginPlay`
  (`SkeletalMeshComponent.PlayAnimation` (`self.SkeletalMesh`) "/Game/Model/taiko_wait.taiko_wait" false)
  (bind _asthird_person_character (cast `/Game/BluePrints/ThirdPersonCharacter` (`GameplayStatics.GetPlayerPawn` 0)))
  (add `/Game/BluePrints/ThirdPersonCharacter.HugTime` _asthird_person_character (delegate `Let'sHug`))
  (add `/Game/BluePrints/ThirdPersonCharacter.HugEnd` _asthird_person_character (delegate `I'mHappy`)))

(event `I'mHappy`
  (set `self.isHug` false)
  (`SkeletalMeshComponent.PlayAnimation` (`self.SkeletalMesh`) "/Game/Model/taiko_shouten.taiko_shouten" false))

(event `Let'sHug`
  (bind _output_get (set `self.isHug` true))
  (`SkeletalMeshComponent.PlayAnimation` (`self.SkeletalMesh`) "/Game/Model/taiko_hagu.taiko_hagu" false))

(event `self.ReceiveTick`
  (params (DeltaSeconds :type "Float (single-precision)"))
  (if (stale `Let'sHug` _output_get)
    (`SceneComponent.K2_SetWorldRotation` (`self.DefaultSceneRoot`) (`KismetMathLibrary.MakeRotator` 0.0 0.0 (- (.yaw (`KismetMathLibrary.FindLookAtRotation` (`SceneComponent.K2_GetComponentLocation` (`self.SkeletalMesh`)) (`self.K2_GetActorLocation` (`GameplayStatics.GetPlayerPawn` 0)))) 90.0)) false false)))

(fn `UserConstructionScript`)