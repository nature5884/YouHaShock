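; Enemy Blueprint that turns to face the player, detects them, and drains their LovePower when in attack range.
; Sphere and Attack overlaps toggle discover and attack flags, which Tick reads to call AIMoveTo or a delayed AttackFunc.
; BeginPlay binds Damage_Event to the player character's hit event to play a flinch animation.
; The chase's AIMoveTo and PlayAnimation calls have no destination or animation set.
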(event `self.ReceiveBeginPlay`
  (bind _asthird_person_character (cast `/Game/BluePrints/ThirdPersonCharacter` (`GameplayStatics.GetPlayerPawn` 0)))
  (add `/Game/BluePrints/ThirdPersonCharacter.HitEvent` _asthird_person_character (delegate `Damage_Event`)))

(event `Damage_Event`
  (`KismetSystemLibrary.PrintString` "damage")
  (`SkeletalMeshComponent.PlayAnimation` (`self.SkeletalMesh`) "/Game/Model/mohiAnim/mohi-_hirumi.mohi-_hirumi" false))

(event `self.ReceiveTick`
  (params (DeltaSeconds :type "Float (single-precision)"))
  (bind _returnvalue (`GameplayStatics.GetPlayerPawn` 0))
  (bind _skeletalmesh (`self.SkeletalMesh`))
  (`|ExecutionSequence`
    (:`then_0`
      (`SceneComponent.K2_SetWorldRotation` _skeletalmesh (`KismetMathLibrary.MakeRotator` 0.0 0.0 (- (.yaw (`KismetMathLibrary.FindLookAtRotation` (`SceneComponent.K2_GetComponentLocation` _skeletalmesh) (`self.K2_GetActorLocation` _returnvalue))) 90.0)) false false))
    (:`then_1`
      (if (`self.isDiscover`)
        (`SkeletalMeshComponent.PlayAnimation` (`self.SkeletalMesh`) null false)
        (`AITask_MoveTo.AIMoveTo` null)))
    (:`then_2`
      (if (`self.isAttack`)
        (`KismetSystemLibrary.Delay` 0.5)
        (`self.AttackFunc` _returnvalue)))))

(event `self.Sphere.OnComponentBeginOverlap`
  (params (OtherActor :type "Actor Object Reference") (OtherComp :type "PrimitiveComponent Object Reference") (OtherBodyIndex :type Integer) (bFromSweep :type Boolean) (SweepResult :type "HitResult Structure (by ref)"))
  (if (== OtherActor (`GameplayStatics.GetPlayerPawn` 0))
    (set `self.isDiscover` true)))

(event `self.Attack.OnComponentBeginOverlap`
  (params (OtherActor :type "Actor Object Reference") (OtherComp :type "PrimitiveComponent Object Reference") (OtherBodyIndex :type Integer) (bFromSweep :type Boolean) (SweepResult :type "HitResult Structure (by ref)"))
  (if (== OtherActor (`GameplayStatics.GetPlayerPawn` 0))
    (set `self.isAttack` true)
    (set `self.isDiscover` false)))

(event `self.Attack.OnComponentEndOverlap`
  (params (OtherActor :type "Actor Object Reference") (OtherComp :type "PrimitiveComponent Object Reference") (OtherBodyIndex :type Integer))
  (if (== OtherActor (`GameplayStatics.GetPlayerPawn` 0))
    (set `self.isAttack` false)
    (set `self.isDiscover` true)))

(fn `AttackFunc`
  (params (Object :type "Object Object Reference"))
  (`KismetSystemLibrary.PrintString` "ヒャッハー！！！" false false)
  (bind _asthird_person_character (cast `/Game/BluePrints/ThirdPersonCharacter` Object)
    (:`then`
      (bind _lovepower (`/Game/BluePrints/ThirdPersonCharacter.LovePower` _asthird_person_character))
      (if (> _lovepower 0)
        (set `/Game/BluePrints/ThirdPersonCharacter.LovePower` (- _lovepower 1) _asthird_person_character)))
    (:`CastFailed`
      _))
  (return))

(fn `UserConstructionScript`)