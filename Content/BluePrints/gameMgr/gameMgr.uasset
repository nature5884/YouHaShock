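; gameMgr is a game manager Blueprint that creates the UI, spawns oases and handles game-over restarts.
; BeginPlay adds the UI widget to the viewport, and GameOver starts a tick-counted countdown that ends by opening GameLevel.
; Tick also increments Hoge, copies it over KillMohiCount despite the separate KillCountUp function, and periodically spawns OasisBP at the first ThirdPersonCharacter's mesh transform.
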(event `self.ReceiveBeginPlay`
  (bind _returnvalue (`|CreateWidget` "/Game/CG/Widget/UIwid.UIwid_C" (`GameplayStatics.GetPlayerController` 0)))
  (`UserWidget.AddToViewport` _returnvalue 0))

(event `self.ReceiveTick`
  (params (DeltaSeconds :type "Float (single-precision)"))
  (`|ExecutionSequence`
    (:`then_0`
      (`self.GameOverCheck`))
    (:`then_1`
      (bind _output_get (set `self.hoge` (+ (`self.hoge`) 1)))
      (set `self.killMohiCount` _output_get)
      (if (== (mod _output_get 100) 0)
        (bind _outactors (`GameplayStatics.GetAllActorsOfClass` "/Game/BluePrints/ThirdPersonCharacter.ThirdPersonCharacter_C"))
        (`|SpawnActorFromClass` "/Game/Blueprints/oasisBP.oasisBP_C" (`SceneComponent.K2_GetComponentToWorld` (`Character.Mesh` (`KismetArrayLibrary.Array_Get` _outactors))) "Undefined" "OverrideRootScale")))))

(fn `GameOver`
  (`KismetSystemLibrary.PrintString` "Hello")
  (set `self.timer` 10)
  (set `self.gameOverFlg` true)
  (return))

(fn `killCountUp`
  (`/Engine/EditorBlueprintResources/StandardMacros.IncrementInt` (`self.killMohiCount`)
    (:`  `
      (return))))

(fn `UserConstructionScript`)