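; Oasis actor that spawns tiny and grows into the world, with a healing particle effect (the "Heart") above it.
; BeginPlay shrinks the actor and spawns the emitter, then Tick steps the actor's scale up to MAXSCALESIZE and keeps enlarging the emitter while active.
; ScaleDown is never called; its comment indicates scaling by the lovers' love level, but it currently multiplies by zero.
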(event `self.ReceiveBeginPlay`
  (`self.SetActorScale3D` (0.01 0.01 0.01))
  (bind _returnvalue (`GameplayStatics.SpawnEmitterAtLocation` "/Game/InfinityBladeEffects/Effects/FX_Ability/Heal/P_Heal_Startup_mobile.P_Heal_Startup_mobile" (`KismetMathLibrary.MakeVector` (.x (`self.K2_GetActorLocation`)) (.y (`self.K2_GetActorLocation`)) (+ (.z (`self.K2_GetActorLocation`)) 100.0))))
  (set `self.heart` _returnvalue))

(event `self.ReceiveActorBeginOverlap`
  (params (OtherActor :type "Actor Object Reference")))

(event `self.ReceiveTick`
  (params (DeltaSeconds :type "Float (single-precision)"))
  (bind _heart (`self.heart`))
  (bind _heart_2 (`self.heart`))
  (`|ExecutionSequence`
    (:`then_0`
      (`self.appearOasis`))
    (:`then_1`
      (if (!= _heart_2 null)
        (if (`ActorComponent.IsActive` _heart_2)
          (`SceneComponent.SetWorldScale3D` _heart (+ (`SceneComponent.K2_GetComponentScale` _heart) 0.01)))))))

(fn `UserConstructionScript`)